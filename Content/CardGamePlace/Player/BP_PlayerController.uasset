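; Player controller for the card game that manages round and block-action UI.
; On BeginPlay it shows the cursor and, for the autonomous proxy only, creates the end-round widget, whose button state updates on round-state changes.
; CreateMyAnnexationWidget hides the block-action widget and opens an annexation widget for a starting block; right-click cancels back to the block-action widget.
; Ending a round removes and clears both block-action and annexation widgets.
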(event `self.ReceiveBeginPlay`
  (set `self.bShowMouseCursor` true)
  (if (`|EnumEquality` (`self.GetLocalRole` self) "ROLE_AutonomousProxy")
    (bind _returnvalue (`|CreateWidget` "/Game/CardGamePlace/UI/EndRoundWidget.EndRoundWidget_C" self self))
    (bind _output_get (set `self.MyEndRoundWidget` _returnvalue))
    (`UserWidget.AddToViewport` _output_get 0)))

(event `self.ReceiveTick`
  (params (DeltaSeconds :type "Float (single-precision)")))

(event `Key|RightMouseButton`
  (params (Key :type "Key Structure"))
  (bind _myannexationwidget (`self.MyAnnexationWidget`))
  (bind _myblockdowidget (`self.MyBlockDoWidget`))
  (:`Pressed`
    (if true
      (if (`KismetSystemLibrary.IsValid` _myannexationwidget)
        (if (`KismetSystemLibrary.IsValid` _myblockdowidget)
          (`Widget.SetVisibility` _myblockdowidget "Visible")
          (`Widget.RemoveFromParent` _myannexationwidget)
          (set `self.MyAnnexationWidget` null)
          (else
            (`KismetSystemLibrary.PrintText` "In BP_PlayerController “My Block Do Widget” is null，it shouldn‘t")))))))

(event `self.BPEndRound`
  (bind _myannexationwidget (`self.MyAnnexationWidget`))
  (bind _myblockdowidget (`self.MyBlockDoWidget`))
  (`/Engine/EditorBlueprintResources/StandardMacros.IsValid` _myannexationwidget
    (:`Is Valid`
      (`Widget.RemoveFromParent` _myannexationwidget)
      (set `self.MyAnnexationWidget` null))
    (:`Is Not Valid`
      _))
  (`/Engine/EditorBlueprintResources/StandardMacros.IsValid` _myblockdowidget
    (:`Is Valid`
      (`Widget.RemoveFromParent` _myblockdowidget)
      (set `self.MyBlockDoWidget` null))))

(event `self.BPChangeRoundState`
  (`/Game/CardGamePlace/UI/EndRoundWidget.ChangeEndRoundButtonState` (`self.MyEndRoundWidget`)))

(fn `CreateMyAnnexationWidget`
  (params (BeginAnnexationBlock :type "ZPlayerBlock Object Reference"))
  (returns (BisSuccess :type Boolean))
  (bind _myblockdowidget (`self.MyBlockDoWidget`))
  (if (`KismetSystemLibrary.IsValid` _myblockdowidget)
    (`Widget.SetVisibility` _myblockdowidget "Hidden")
    (bind _returnvalue (`|CreateWidget` "/Game/CardGamePlace/UI/DoAnnexationWidget.DoAnnexationWidget_C" null BeginAnnexationBlock self))
    (bind _output_get (set `self.MyAnnexationWidget` _returnvalue))
    (`UserWidget.SetPositionInViewport` _output_get (0.0 0.0) true)
    (`UserWidget.AddToViewport` _output_get 0)
    (return true)))

(fn `UserConstructionScript`)