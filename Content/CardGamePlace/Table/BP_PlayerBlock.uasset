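; BP_PlayerBlock is a clickable, player-owned grid block on the card game table that handles expansion and annexation input.
; On the player's round, clicking toggles an action menu at the mouse, opened only on owned blocks.
; During annexation, hover asks the controller's annexation widget to validate the target, and clicking a valid one has the origin block annex it, then clears both widgets.
; Debug prints remain throughout, including on Tick.
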(event `self.ReceiveBeginPlay`
  ;[1 1 1] debug for place
  (bind _asbp_player_controller (cast `/Game/CardGamePlace/Player/BP_PlayerController` (`GameplayStatics.GetPlayerController` 0)))
  (set `self.BPPlayerController` _asbp_player_controller)
  (`KismetSystemLibrary.PrintString` (`KismetStringLibrary.Concat_StrStr` (`KismetStringLibrary.Conv_IntToString` (`self.GridY`)) (`KismetStringLibrary.Conv_IntToString` (`self.GridX`)))))

(event `self.MeshComponent.OnClicked`
  (params (TouchedComponent :type "PrimitiveComponent Object Reference") (ButtonPressed :type "Key Structure"))
  (bind _bpplayercontroller (`self.BPPlayerController`))
  (bind _bpplayercontroller_2 (`self.BPPlayerController`))
  (bind _myblockdowidget (`/Game/CardGamePlace/Player/BP_PlayerController.MyBlockDoWidget` _bpplayercontroller))
  (bind _myannexationwidget (`/Game/CardGamePlace/Player/BP_PlayerController.MyAnnexationWidget` _bpplayercontroller_2))
  (bind _beginannexationblock (`/Game/CardGamePlace/UI/DoAnnexationWidget.BeginAnnexationBlock` _myannexationwidget))
  (if (`ZPlayerController.BisMyRound` (`self.BPPlayerController`))
    (if (`KismetSystemLibrary.IsValid` _bpplayercontroller_2)
      (if (`KismetSystemLibrary.IsValid` _myannexationwidget)
        (if (`/Game/CardGamePlace/UI/DoAnnexationWidget.BisPlayBlockForAnnexation` _myannexationwidget)
          (`KismetSystemLibrary.PrintString` (`KismetSystemLibrary.GetDisplayName` _beginannexationblock) false)
          (`self.DoServeActionAnnexation` _beginannexationblock self)
          (`self.AfterAnnexation`))
        (else
          ;[1 1 1] 扩张和吞并的执行UI创建
          (if (`KismetSystemLibrary.IsValid` _myblockdowidget)
            (if (`Widget.IsVisible` _myblockdowidget)
              (`Widget.RemoveFromParent` _myblockdowidget)
              (set `/Game/CardGamePlace/Player/BP_PlayerController.MyBlockDoWidget` null _bpplayercontroller))
            (elif (== (`ZPlayerController.PlayerControllerID` _bpplayercontroller) (`self.PlayerOwner`))
              (`|ExecutionSequence`
                (:`then_0`
                  (bind _returnvalue (`WidgetLayoutLibrary.GetMousePositionOnViewport`)))
                (:`then_1`
                  (bind _returnvalue_2 (`|CreateWidget` "/Game/CardGamePlace/UI/BlockDoWidget.BlockDoWidget_C" (`GameplayStatics.GetPlayerController` 0) self))
                  (set `/Game/CardGamePlace/Player/BP_PlayerController.MyBlockDoWidget` _returnvalue_2 (`self.BPPlayerController`))
                  (`UserWidget.SetPositionInViewport` _returnvalue_2 _returnvalue false)
                  (`UserWidget.AddToViewport` _returnvalue_2 0))))))))))

(event `self.ReceiveTick`
  (params (DeltaSeconds :type "Float (single-precision)"))
  (`KismetSystemLibrary.PrintString` (`KismetStringLibrary.Conv_BoolToString` (`ZPlayerController.BisMyRound` (`self.BPPlayerController`))) true true (struct :`G` 0.66 :`B` 1.0 :`A` 1.0) 0.0))

(event `self.MeshComponent.OnBeginCursorOver`
  (params (TouchedComponent :type "PrimitiveComponent Object Reference"))
  (bind _bpplayercontroller (`self.BPPlayerController`))
  (bind _myannexationwidget (`/Game/CardGamePlace/Player/BP_PlayerController.MyAnnexationWidget` _bpplayercontroller))
  ;[1 1 1] 判断是否可以吞并
  (if (`KismetSystemLibrary.IsValid` _bpplayercontroller)
    (if (`KismetSystemLibrary.IsValid` _myannexationwidget)
      (bind _result (`/Game/CardGamePlace/UI/DoAnnexationWidget.JudgeForAnnexation` _myannexationwidget self))
      (if _result
        (`KismetSystemLibrary.PrintString` "fuck")))
    (else
      (`KismetSystemLibrary.PrintText` "In BP_PlayerBlock ZPlayerController is null"))))

(event `self.MeshComponent.OnEndCursorOver`
  (params (TouchedComponent :type "PrimitiveComponent Object Reference"))
  (bind _myannexationwidget (`/Game/CardGamePlace/Player/BP_PlayerController.MyAnnexationWidget` (`self.BPPlayerController`)))
  (bind _currentcursoroverplayerblock (`/Game/CardGamePlace/UI/DoAnnexationWidget.CurrentCursorOverPlayerBlock` _myannexationwidget))
  ;[1 1 1] 重置吞并状态
  (if (`KismetSystemLibrary.IsValid` _myannexationwidget)
    (if (`KismetSystemLibrary.IsValid` _currentcursoroverplayerblock)
      (if (== _currentcursoroverplayerblock self)
        (set `/Game/CardGamePlace/UI/DoAnnexationWidget.BisPlayBlockForAnnexation` false _myannexationwidget)))))

(fn `AfterAnnexation`
  (bind _asbp_player_controller (cast `/Game/CardGamePlace/Player/BP_PlayerController` (`self.BPPlayerController`)))
  (bind _myannexationwidget (`/Game/CardGamePlace/Player/BP_PlayerController.MyAnnexationWidget` _asbp_player_controller))
  (`/Engine/EditorBlueprintResources/StandardMacros.IsValid` _myannexationwidget
    (:`Is Valid`
      (`Widget.RemoveFromParent` _myannexationwidget)
      (bind _myblockdowidget (`/Game/CardGamePlace/Player/BP_PlayerController.MyBlockDoWidget` _asbp_player_controller))
      (`/Engine/EditorBlueprintResources/StandardMacros.IsValid` _myblockdowidget
        (:`Is Valid`
          (`Widget.RemoveFromParent` _myblockdowidget)
          (set `/Game/CardGamePlace/Player/BP_PlayerController.MyAnnexationWidget` null _asbp_player_controller)
          (set `/Game/CardGamePlace/Player/BP_PlayerController.MyBlockDoWidget` null _asbp_player_controller))))))

(fn `UserConstructionScript`)